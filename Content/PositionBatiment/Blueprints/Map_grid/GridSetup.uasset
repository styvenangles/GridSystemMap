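; GridSetup builds the map grid at BeginPlay by spawning Grid_Base actors in a GridX by GridY layout.
; A nested loop spaces the cells by GridSize and offsets them by half the grid's extent, roughly centering them on this actor's location.
; Each spawned cell is unrotated, at unit scale, and stored in GridBaseArray.
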(event `self.ReceiveBeginPlay`
  (bind _grid_x (`self.Grid_X`))
  (bind _grid_y (`self.Grid_Y`))
  (bind _grid_size (`self.Grid_Size`))
  (for _index (range 1 (+ _grid_x 1))
    (for _index_2 (range 1 (+ _grid_y 1))
      (bind _returnvalue (`|SpawnActorFromClass` "/Game/PositionBatiment/Blueprints/Map_grid/Grid_Base.Grid_Base_C" (`KismetMathLibrary.MakeTransform` (+ (`KismetMathLibrary.MakeVector` (`KismetMathLibrary.Conv_IntToDouble` (- (* _index _grid_size) (/ (* _grid_x _grid_size) 2))) (`KismetMathLibrary.Conv_IntToDouble` (- (* _index_2 _grid_size) (/ (* _grid_y _grid_size) 2)))) (`self.K2_GetActorLocation`))) "Undefined" "OverrideRootScale" null null))
      (`KismetArrayLibrary.Array_Add` (`self.GridBaseArray`) _returnvalue))))

(fn `UserConstructionScript`)