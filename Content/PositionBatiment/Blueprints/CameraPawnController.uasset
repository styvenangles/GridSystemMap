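; Player controller for a building-placement game that drives a camera pawn and starts building construction.
; BeginPlay caches the pawn, creates the main HUD, and spawns the construction manager and ghost building actors.
; Forward input, unless navigation is disabled, moves the camera at a speed derived from clamped spring-arm length.
; ConstructBuilding spawns the requested building and resets the ghost, passing it the display mesh, class and construction proxy.
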(event `self.ReceiveBeginPlay`
  (bind _returnvalue (`KismetMathLibrary.MakeTransform` (0.0 0.0 0.0)))
  ;[1 1 1] BeginPlay
  (`|ExecutionSequence`
    (:`then_0`
      (`self.ReferenceCasts`))
    (:`then_1`
      (`WidgetBlueprintLibrary.SetInputMode_GameAndUIEx` self null "LockAlways" false)
      (`self.CreateHuds`)
      (`UserWidget.AddToViewport` (`self.MainHudRef`) 0))
    (:`then_2`
      (bind _returnvalue_2 (`|SpawnActorFromClass` "/Game/PositionBatiment/Blueprints/Constructions/ConstructionManager_BP.ConstructionManager_BP_C" _returnvalue "AlwaysSpawn" "OverrideRootScale" null null))
      (set `self.ConstructionManagerRef` _returnvalue_2))
    (:`then_3`
      (bind _returnvalue_3 (`|SpawnActorFromClass` "/Game/PositionBatiment/Blueprints/Buildings/GhostBuilding_BP.GhostBuilding_BP_C" _returnvalue "AlwaysSpawn" "OverrideRootScale" null self null))
      (set `self.GhostBuildingRef` _returnvalue_3))))

(event `InputAxis|MoveForward`
  (params (AxisValue :type "Float (single-precision)"))
  ;[1 1 1] CameraController
  (if (not (`self.DisableCamNav`))
    (`self.K2_SetActorTransform` (`self.CameraPawnRef`) (`self.MvtX` (`self.MvtSpeedCalc`) (`self.FastMoveMultiplier`) AxisValue (`self.CameraPawnRef`)) false false)))

(event `/Game/PositionBatiment/Interfaces/I_HUD.ConstructBuilding`
  (params (MainBuilding :type "/Game/PositionBatiment/Blueprints/Buildings/BuildingMaster_BP Class Reference"))
  (bind _ghostbuildingref (`self.GhostBuildingRef`))
  (bind _returnvalue (`|SpawnActorFromClass` MainBuilding (`KismetMathLibrary.MakeTransform` (0.0 0.0 0.0)) "Undefined" "OverrideRootScale" null self null))
  (bind _asbuilding_master_bp (castclass `/Game/PositionBatiment/Blueprints/Buildings/BuildingMaster_BP` MainBuilding))
  (`/Game/PositionBatiment/Blueprints/Buildings/GhostBuilding_BP.KillGhost` _ghostbuildingref)
  (`/Game/PositionBatiment/Blueprints/Buildings/GhostBuilding_BP.OnSpawn` _ghostbuildingref (`/Game/PositionBatiment/Blueprints/Buildings/BuildingMaster_BP.DisplayMesh` _returnvalue) _asbuilding_master_bp (`/Game/PositionBatiment/Blueprints/Buildings/BuildingMaster_BP.ConstructionProxy` _returnvalue)))

(fn `MvtSpeedCalc`
  (returns (MoveSensitivity :type "Float (double-precision)"))
  (return (`KismetMathLibrary.FClamp` (/ (`SpringArmComponent.TargetArmLength` (`/Game/PositionBatiment/Blueprints/CameraPawn.SpringArm` (`self.CameraPawnRef`))) 100.0) 5.0 20.0)))

(fn `UserConstructionScript`)